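; Pushable block Blueprint that visually indicates which side is highlighted and which side it is being pushed to.
; Tick shows MovingAnimation while IsMoving is set, rotated to the stored BlockSide, and clears any highlight.
; HighlightSide briefly shows HighlightedAnimation on the given side, then hides it after a short delay.
; PushToSide only records the side, and GetAngleForSide maps each side to a world rotation in quarter turns.
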(event `self.ReceiveTick`
  (params (DeltaSeconds :type "Float (single-precision)"))
  (bind _movinganimation (`self.MovingAnimation`))
  (if (`self.IsMoving`)
    (`SceneComponent.SetVisibility` _movinganimation true false)
    (bind _rotation (`self.GetAngleForSide` (`self.BlockSide`)))
    (`SceneComponent.K2_SetWorldRotation` (`self.MovingAnimation`) _rotation false false)
    (`self.ClearHighlight`)
    (else
      (`SceneComponent.SetVisibility` _movinganimation false false))))

(event `HighlightSide`
  (params (Side :type "EBlockSide Enum" :default "Front"))
  (`SceneComponent.SetVisibility` (`self.HighlightedAnimation`) true false)
  (bind _rotation (`self.GetAngleForSide` Side))
  (`SceneComponent.K2_SetWorldRotation` (`self.HighlightedAnimation`) _rotation false false)
  (`KismetSystemLibrary.Delay` 0.05)
  (`self.ClearHighlight`))

(event `ClearHighlight`
  (`SceneComponent.SetVisibility` (`self.HighlightedAnimation`) false false))

(event `PushToSide`
  (params (Blockside :type "EBlockSide Enum" :default "Front"))
  (set `self.BlockSide` Blockside))

(fn `GetAngleForSide`
  (params (Side :type "EBlockSide Enum" :default "Front"))
  (returns (Rotation :type "Rotator Structure"))
  (switch `EBlockSide` Side
    (:`Front`
      (return))
    (:`Left`
      (return (struct :`Yaw` 270.0)))
    (:`Back`
      (return (struct :`Yaw` 180.0)))
    (:`Right`
      (return (struct :`Yaw` 90.0)))))

(fn `UserConstructionScript`)